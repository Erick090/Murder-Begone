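; WineGlas_BP is a wine glass actor that drives an outline glow on its mesh when the MurdererScript actor overlaps its UITrigger.
; The HintGlas flag selects one of two timelines, each feeding the glow power parameter of a newly created dynamic material instance.
; Each timeline writes HintGlas back to the value that selected it, so the flag never toggles here.
; End overlap only casts and has no effect.
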(event `self.UI Trigger.OnComponentBeginOverlap`
  (params (OverlappedComponent :type "PrimitiveComponent Object Reference") (OtherActor :type "Actor Object Reference") (OtherComp :type "PrimitiveComponent Object Reference") (OtherBodyIndex :type Integer) (bFromSweep :type Boolean) (SweepResult :type "HitResult Structure (by ref)"))
  (cast `/Game/Blueprints/Character/MurdererScript` OtherActor)
  (if (`self.Hint_Glas`)
    (bind _returnvalue (`PrimitiveComponent.CreateDynamicMaterialInstance` (`self.Glass`) 0 null))
    (bind (_direction _newtrack_0) (`Timeline|Timeline_0`)
      (:`Update`
        (`MaterialInstanceDynamic.SetScalarParameterValue` _returnvalue "OutlineGlowPower (S)" _newtrack_0)
        (set `self.Hint_Glas` true)))
    (else
      (bind _returnvalue_2 (`PrimitiveComponent.CreateDynamicMaterialInstance` (`self.Glass`) 0 null))
      (bind (_direction_2 _newtrack_0_2) (`Timeline|Timeline_1`)
        (:`Update`
          (`MaterialInstanceDynamic.SetScalarParameterValue` _returnvalue_2 "OutlineGlowPower (S)" _newtrack_0_2)
          (set `self.Hint_Glas` false))))))

(event `self.UI Trigger.OnComponentEndOverlap`
  (params (OverlappedComponent :type "PrimitiveComponent Object Reference") (OtherActor :type "Actor Object Reference") (OtherComp :type "PrimitiveComponent Object Reference") (OtherBodyIndex :type Integer))
  (cast `/Game/Blueprints/Character/MurdererScript` OtherActor))

(fn `UserConstructionScript`)