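; ObjA is a prototype interactable actor with a UITrigger component, apparently built to test input and event dispatchers.
; Its only active logic sets AmIHolding while the TestActionV input is held and clears it on release.
; Overlap and hit events are empty, and disconnected leftover nodes hold MurdererScript casts, debug prints and an ObjADispatcher call that never runs.
; The construction script and GetObject function do nothing.
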(event `self.ReceiveActorBeginOverlap`
  (params (OtherActor :type "Actor Object Reference")))

(event `self.ReceiveHit`
  (params (MyComp :type "PrimitiveComponent Object Reference") (Other :type "Actor Object Reference") (OtherComp :type "PrimitiveComponent Object Reference") (bSelfMoved :type Boolean) (HitLocation :type "Vector Structure") (HitNormal :type "Vector Structure") (NormalImpulse :type "Vector Structure") (Hit :type "HitResult Structure (by ref)")))

(event `self.UI Trigger.OnComponentBeginOverlap`
  (params (OverlappedComponent :type "PrimitiveComponent Object Reference") (OtherActor :type "Actor Object Reference") (OtherComp :type "PrimitiveComponent Object Reference") (OtherBodyIndex :type Integer) (bFromSweep :type Boolean) (SweepResult :type "HitResult Structure (by ref)")))

(event `self.UI Trigger.OnComponentHit`
  (params (HitComponent :type "PrimitiveComponent Object Reference") (OtherActor :type "Actor Object Reference") (OtherComp :type "PrimitiveComponent Object Reference") (NormalImpulse :type "Vector Structure") (Hit :type "HitResult Structure (by ref)")))

(event `InputAction|TestActionV`
  (params (Key :type "Key Structure"))
  (:`Pressed`
    (set `self.AmIHolding` true))
  (:`Released`
    (set `self.AmIHolding` false)))

(fn `GetObject`
  (if true
    _))

(fn `UserConstructionScript`)