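; MainGameMode is a game mode Blueprint that starts the background music when play begins.
; BeginPlay plays the Hintergrundmusik sound at the world origin through PlaySoundAtLocation.
; A count-up clock that would add seconds after a one-second delay and roll them into minutes is present but disconnected, so it never runs.
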(event `self.ReceiveBeginPlay`
  (`|ExecutionSequence`
    (:`then_0`
      (`GameplayStatics.PlaySoundAtLocation` "/Game/Audio/Enviroment/Hintergrundmusik.Hintergrundmusik"))))

(fn `UserConstructionScript`)