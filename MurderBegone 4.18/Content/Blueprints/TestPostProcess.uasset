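; Test trigger actor that toggles a post process effect and camera zoom when something enters or leaves its box.
; Box begin overlap sets the TestPP blend radius to 10 and narrows the MurdererScript player camera's field of view to 45.
; End overlap resets the radius to zero and the field of view to 90, printing debug text on each change.
; The overlapping actor is never checked, so any overlap affects player zero.
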(event `self.Box.OnComponentBeginOverlap`
  (params (OverlappedComponent :type "PrimitiveComponent Object Reference") (OtherActor :type "Actor Object Reference") (OtherComp :type "PrimitiveComponent Object Reference") (OtherBodyIndex :type Integer) (bFromSweep :type Boolean) (SweepResult :type "HitResult Structure (by ref)"))
  (set `PostProcessComponent.BlendRadius` 10.0 (`self.testPP`))
  (`KismetSystemLibrary.PrintString` "Blend Radius 10")
  (bind _asmurderer_script (cast `/Game/Blueprints/Character/MurdererScript` (`GameplayStatics.GetPlayerCharacter` 0)))
  (`CameraComponent.SetFieldOfView` (`/Game/Blueprints/Character/MurdererScript.Camera` _asmurderer_script) 45.0))

(event `self.Box.OnComponentEndOverlap`
  (params (OverlappedComponent :type "PrimitiveComponent Object Reference") (OtherActor :type "Actor Object Reference") (OtherComp :type "PrimitiveComponent Object Reference") (OtherBodyIndex :type Integer))
  (set `PostProcessComponent.BlendRadius` 0.0 (`self.testPP`))
  (`KismetSystemLibrary.PrintString` "Blend Radius 0" true true (struct :`R` 1.0 :`G` 0.205431 :`B` 0.165626 :`A` 1.0))
  (bind _asmurderer_script (cast `/Game/Blueprints/Character/MurdererScript` (`GameplayStatics.GetPlayerCharacter` 0)))
  (`CameraComponent.SetFieldOfView` (`/Game/Blueprints/Character/MurdererScript.Camera` _asmurderer_script) 90.0))

(fn `UserConstructionScript`)