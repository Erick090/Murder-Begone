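; Bleach prop that the player combines with the knife to bleach it.
; Box overlap enables player input and opens a never-closed gate; E passes through it, casts the overlapping actor to Knife_BP and calls BleachingKnife once.
; Leaving the box disables input.
; Tick reads Glowiness on MurdererScript and plays one of two timelines to drive a hint outline glow, creating a dynamic material instance each frame.
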(event `self.Box.OnComponentBeginOverlap`
  (params (OverlappedComponent :type "PrimitiveComponent Object Reference") (OtherActor :type "Actor Object Reference") (OtherComp :type "PrimitiveComponent Object Reference") (OtherBodyIndex :type Integer) (bFromSweep :type Boolean) (SweepResult :type "HitResult Structure (by ref)"))
  ;[1 1 1] Combination only possible in triggerbox
  (`self.EnableInput` (`GameplayStatics.GetPlayerController` 0))
  (goto _label :!via `Open`))

(event `self.Box.OnComponentEndOverlap`
  (params (OverlappedComponent :type "PrimitiveComponent Object Reference") (OtherActor :type "Actor Object Reference") (OtherComp :type "PrimitiveComponent Object Reference") (OtherBodyIndex :type Integer))
  ;[1 1 1] Combination only possible in triggerbox
  (`self.DisableInput` (`GameplayStatics.GetPlayerController` 0)))

(event `Key|E`
  (params (Key :type "Key Structure"))
  ;[1 1 1] cast to knifBP for anim/Counter etc
  (:`Pressed`
    (`/Engine/EditorBlueprintResources/StandardMacros.Gate` true :!label _label
      (:`Exit`
        (bind _asknife_bp (cast `/Game/Blueprints/Assets/Knife_BP` (stale `self.Box.OnComponentBeginOverlap` OtherActor)))
        (`/Engine/EditorBlueprintResources/StandardMacros.DoOnce` false
          (:`Completed`
            (`/Game/Blueprints/Assets/Knife_BP.BleachingKnife` _asknife_bp)
            (`KismetSystemLibrary.PrintString` "bleach combined" true true (struct :`G` 0.66 :`B` 1.0 :`A` 1.0) 5.0)))))))

(event `self.ReceiveTick`
  (params (DeltaSeconds :type "Float (single-precision)"))
  (bind _asmurderer_script (cast `/Game/Blueprints/Character/MurdererScript` (`GameplayStatics.GetPlayerCharacter` 0)))
  (if (`/Game/Blueprints/Character/MurdererScript.Glowiness` _asmurderer_script)
    ;[1 1 1] activate Hint_Glow
    (bind _returnvalue (`PrimitiveComponent.CreateDynamicMaterialInstance` (`self.bleach_low`) 0 null))
    (bind (_direction _newtrack_0) (`Timeline|Timeline_0`)
      (:`Update`
        (`MaterialInstanceDynamic.SetScalarParameterValue` _returnvalue "OutlineGlowPower (S)" _newtrack_0)))
    (else
      ;[1 1 1] deactivate Hint_Glow
      (bind _returnvalue_2 (`PrimitiveComponent.CreateDynamicMaterialInstance` (`self.bleach_low`) 0 null))
      (bind (_direction_2 _newtrack_0_2) (`Timeline|Timeline_1`)
        (:`Update`
          (`MaterialInstanceDynamic.SetScalarParameterValue` _returnvalue_2 "OutlineGlowPower (S)" _newtrack_0_2))))))

(fn `UserConstructionScript`)