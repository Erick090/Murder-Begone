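; Corpse actor that lets the player press E nearby to hear a one-time "what happened" self-voice line.
; Any actor overlap prints a debug string, enables input for player 0 and opens a gate that never closes.
; E passes through that gate into a DoOnce that plays the 2D sound.
; End overlap disables input when the CorpseCollider overlap check fails; the MurdererScript casts are unconnected.
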(event `self.ReceiveActorEndOverlap`
  (params (OtherActor :type "Actor Object Reference"))
  (if (not (`PrimitiveComponent.IsOverlappingComponent` (`self.CorpseCollider`) null))
    (`self.DisableInput` (`GameplayStatics.GetPlayerController` 0))))

(event `Key|E`
  (params (Key :type "Key Structure"))
  (:`Pressed`
    (`/Engine/EditorBlueprintResources/StandardMacros.Gate` true :!label _label
      (:`Exit`
        (`/Engine/EditorBlueprintResources/StandardMacros.DoOnce` false
          (:`Completed`
            (`GameplayStatics.PlaySound2D` "/Game/Audio/VoiceOver/Murder_Begone_SelfVoice_whatHappend_master.Murder_Begone_SelfVoice_whatHappend_master")))))))

(event `self.ReceiveActorBeginOverlap`
  (params (OtherActor :type "Actor Object Reference"))
  (`KismetSystemLibrary.PrintText` "Corpse?")
  (`self.EnableInput` (`GameplayStatics.GetPlayerController` 0))
  (goto _label :!via `Open`))

(fn `UserConstructionScript`)