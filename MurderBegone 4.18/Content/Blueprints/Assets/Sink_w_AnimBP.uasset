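; Interactive sink actor that runs a timed tap sequence and lets the knife be washed.
; UITrigger overlap enables input and opens a gate, so E plays a level sequence, tap animation and sounds, with delays toggling water visibility on and off.
; The first run sets IsTapOpen, which is never reset here.
; While it is true, a Knife_BP overlapping the Capsule triggers WashingKnife through a DoOnce.
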(event `Key|E`
  (params (Key :type "Key Structure"))
  ;[1 1 1] Overlap_Trigger and Press "E"
  (:`Pressed`
    (`/Engine/EditorBlueprintResources/StandardMacros.Gate` true :!label _label
      (:`Exit`
        ;[1 1 1] Tap_Animation_and_Sequence
        (`|ExecutionSequence`
          (:`then_0`
            (`MovieSceneSequencePlayer.Play` (`LevelSequenceActor.SequencePlayer` (`self.Sink_Sequence`)))
            (`AudioComponent.Play` (`self.Tab`) 0.0)
            (`SkeletalMeshComponent.PlayAnimation` (`self.Sink_new`) "/Game/VFX/Sink/Anim/Sink_new_TabClose_Anim.Sink_new_TabClose_Anim" false)
            (`KismetSystemLibrary.Delay` 3.3333)
            (`SceneComponent.ToggleVisibility` (`self.Sink_water`) false)
            (set `self.IsTapOpen` true)
            (`AudioComponent.Play` (`self.Water_Start`) 0.0)
            (`KismetSystemLibrary.Delay` 5.0)
            (`AudioComponent.Play` (`self.Tab`) 0.0)
            (`SkeletalMeshComponent.PlayAnimation` (`self.Sink_new`) "/Game/VFX/Sink/Anim/Sink_new_TabClose_Anim.Sink_new_TabClose_Anim" false)
            (`AudioComponent.Play` (`self.Water_End`) 0.0)
            (`KismetSystemLibrary.Delay` 3.3333)
            (`SceneComponent.ToggleVisibility` (`self.Sink_water`) false)
            (`AudioComponent.Stop` (`self.Water_Start`))))))))

(event `self.UI Trigger.OnComponentBeginOverlap`
  (params (OverlappedComponent :type "PrimitiveComponent Object Reference") (OtherActor :type "Actor Object Reference") (OtherComp :type "PrimitiveComponent Object Reference") (OtherBodyIndex :type Integer) (bFromSweep :type Boolean) (SweepResult :type "HitResult Structure (by ref)"))
  ;[1 1 1] Overlap_Trigger and Press "E"
  (`self.EnableInput` (`GameplayStatics.GetPlayerController` 0))
  (goto _label :!via `Open`))

(event `self.UI Trigger.OnComponentEndOverlap`
  (params (OverlappedComponent :type "PrimitiveComponent Object Reference") (OtherActor :type "Actor Object Reference") (OtherComp :type "PrimitiveComponent Object Reference") (OtherBodyIndex :type Integer))
  ;[1 1 1] Overlap_Trigger and Press "E"
  (`self.DisableInput` (`GameplayStatics.GetPlayerController` 0)))

(event `self.Capsule.OnComponentBeginOverlap`
  (params (OverlappedComponent :type "PrimitiveComponent Object Reference") (OtherActor :type "Actor Object Reference") (OtherComp :type "PrimitiveComponent Object Reference") (OtherBodyIndex :type Integer) (bFromSweep :type Boolean) (SweepResult :type "HitResult Structure (by ref)"))
  ;[1 1 1] wenn knife and water overlap -> event washing knife in knifeBP
  (if (`self.IsTapOpen`)
    (bind _asknife_bp (cast `/Game/Blueprints/Assets/Knife_BP` OtherActor))
    (`/Engine/EditorBlueprintResources/StandardMacros.DoOnce` false
      (:`Completed`
        (`/Game/Blueprints/Assets/Knife_BP.WashingKnife` _asknife_bp)
        (`KismetSystemLibrary.PrintString` "cast to knife BP")))))

(event `Key|E`
  (params (Key :type "Key Structure"))
  ;[1 1 1] sfx of water in sink (inactive)
)

(fn `UserConstructionScript`)