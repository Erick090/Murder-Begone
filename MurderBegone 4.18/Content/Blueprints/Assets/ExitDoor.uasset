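; Exit door actor that offers the player an exit confirmation dialog when clicked from within its trigger.
; Any actor overlap prints an exit prompt, enables input on the door and opens a gate that is never explicitly closed.
; A left click through the gate shows the ConfirmExit widget with mouse cursor and UI-only input, leaving the game unpaused.
; Ending overlap disables door input once DoorCollision overlaps nothing.
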(event `self.ReceiveActorEndOverlap`
  (params (OtherActor :type "Actor Object Reference"))
  ;[1 1 1] Interaction Possible within triggerbox
  (if (not (`PrimitiveComponent.IsOverlappingComponent` (`self.DoorCollision`) null))
    (`self.DisableInput` (`GameplayStatics.GetPlayerController` 0))))

(event `Key|LeftMouseButton`
  (params (Key :type "Key Structure"))
  (bind _returnvalue (`GameplayStatics.GetPlayerController` 0))
  ;[1 1 1] Interaction Possible within triggerbox
  (:`Pressed`
    (`/Engine/EditorBlueprintResources/StandardMacros.Gate` true :!label _label
      (:`Exit`
        ;[1 1 1] Dialouge called
        (bind _returnvalue_2 (`|CreateWidget` "/Game/Blueprints/UI/ConfirmExit.ConfirmExit_C"))
        (`UserWidget.AddToViewport` _returnvalue_2 0)
        (set `PlayerController.bShowMouseCursor` true _returnvalue)
        (`GameplayStatics.SetGamePaused` false)
        (`WidgetBlueprintLibrary.SetInputMode_UIOnlyEx` _returnvalue)))))

(event `self.ReceiveActorBeginOverlap`
  (params (OtherActor :type "Actor Object Reference"))
  ;[1 1 1] Interaction Possible within triggerbox
  (`KismetSystemLibrary.PrintText` "Exit ?")
  (`self.EnableInput` (`GameplayStatics.GetPlayerController` 0))
  (goto _label :!via `Open`))

(fn `UserConstructionScript`)