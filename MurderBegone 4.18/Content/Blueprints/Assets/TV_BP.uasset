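; Interactive television that the player toggles on and off with E while inside its UITrigger volume.
; Overlapping the trigger enables input and opens a gate; ScreenSwitch then selects timelines that drive Emissive_Power on dynamic material instances of the base and screen.
; Switching on also fades in TVCue, as does the actor begin-overlap event, which replays the screen-on timeline.
; Actor end-overlap fades the sound out, while switching off leaves it untouched.
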(event `Key|E`
  (params (Key :type "Key Structure"))
  ;[1 1 1] Overlap_Trigger and Press "E"
  (:`Pressed`
    (`/Engine/EditorBlueprintResources/StandardMacros.Gate` true :!label _label
      (:`Exit`
        (if (`self.ScreenSwitch`)
          ;[1 1 1] TV_Off
          (`|ExecutionSequence`
            (:`then_0`
              (bind _returnvalue (`PrimitiveComponent.CreateDynamicMaterialInstance` (`self.TV_Base`) 0 null))
              (bind (_direction _newtrack_0) (`Timeline|Timeline_0`)
                (:`Update`
                  (`MaterialInstanceDynamic.SetScalarParameterValue` _returnvalue "Emissive_Power" _newtrack_0))))
            (:`then_1`
              (bind _returnvalue_2 (`PrimitiveComponent.CreateDynamicMaterialInstance` (`self.TV_Screen`) 0 null))
              (bind (_direction_2 _newtrack_0_2) (`Timeline|Timeline_1`)
                (:`Update`
                  (`MaterialInstanceDynamic.SetScalarParameterValue` _returnvalue_2 "Emissive_Power" _newtrack_0_2)
                  (set `self.ScreenSwitch` false)))))
          (else
            ;[1 1 1] TV_On
            (`|ExecutionSequence`
              (:`then_0`
                (bind _returnvalue_3 (`PrimitiveComponent.CreateDynamicMaterialInstance` (`self.TV_Base`) 0 null))
                (bind (_direction_3 _newtrack_0_3) (`Timeline|Timeline_2`)
                  (:`Update`
                    (`MaterialInstanceDynamic.SetScalarParameterValue` _returnvalue_3 "Emissive_Power" _newtrack_0_3))))
              (:`then_1`
                (bind _returnvalue_4 (`PrimitiveComponent.CreateDynamicMaterialInstance` (`self.TV_Screen`) 0 null))
                (bind (_direction_4 _newtrack_0_4) (`Timeline|Timeline_3` :!label _label_2)
                  (:`Update`
                    (`MaterialInstanceDynamic.SetScalarParameterValue` _returnvalue_4 "Emissive_Power" _newtrack_0_4)
                    (set `self.ScreenSwitch` true))))
              (:`then_2`
                (`AudioComponent.FadeIn` (`self.TV_Cue`) 0.0 1.0 0.0 :!label _label_3)
                (goto _label_2)))))))))

(event `self.UI Trigger.OnComponentBeginOverlap`
  (params (OverlappedComponent :type "PrimitiveComponent Object Reference") (OtherActor :type "Actor Object Reference") (OtherComp :type "PrimitiveComponent Object Reference") (OtherBodyIndex :type Integer) (bFromSweep :type Boolean) (SweepResult :type "HitResult Structure (by ref)"))
  ;[1 1 1] Overlap_Trigger and Press "E"
  (`self.EnableInput` (`GameplayStatics.GetPlayerController` 0))
  (goto _label :!via `Open`))

(event `self.UI Trigger.OnComponentEndOverlap`
  (params (OverlappedComponent :type "PrimitiveComponent Object Reference") (OtherActor :type "Actor Object Reference") (OtherComp :type "PrimitiveComponent Object Reference") (OtherBodyIndex :type Integer))
  ;[1 1 1] Overlap_Trigger and Press "E"
  (`self.DisableInput` (`GameplayStatics.GetPlayerController` 0)))

(event `OnActorBeginOverlap_Event_0`
  (params (OverlappedActor :type "Actor Object Reference") (OtherActor :type "Actor Object Reference"))
  ;[1 1 1] TV_On
  (goto _label_3))

(event `self.ReceiveActorEndOverlap`
  (params (OtherActor :type "Actor Object Reference"))
  (`AudioComponent.FadeOut` (`self.TV_Cue`) 0.0 0.0))

(fn `UserConstructionScript`)