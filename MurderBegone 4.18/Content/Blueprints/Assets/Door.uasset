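; Exit door actor that lets the player leave through a confirmation prompt.
; Any actor overlap prints "Exit ?", enables player input and opens a gate; ending overlap disables input after a DoorCollision check, leaving the gate open.
; Left-click through the gate shows the ConfirmExit widget with cursor and UI-only input, unpaused, and plays a "get out" voice line once.
; The MurdererScript casts are unconnected.
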(event `self.ReceiveActorEndOverlap`
  (params (OtherActor :type "Actor Object Reference"))
  (if (not (`PrimitiveComponent.IsOverlappingComponent` (`self.DoorCollision`) null))
    (`self.DisableInput` (`GameplayStatics.GetPlayerController` 0))))

(event `Key|LeftMouseButton`
  (params (Key :type "Key Structure"))
  (bind _returnvalue (`GameplayStatics.GetPlayerController` 0))
  (:`Pressed`
    (`/Engine/EditorBlueprintResources/StandardMacros.Gate` true :!label _label
      (:`Exit`
        (`|ExecutionSequence`
          (:`then_0`
            (bind _returnvalue_2 (`|CreateWidget` "/Game/Blueprints/UI/ConfirmExit.ConfirmExit_C"))
            (`UserWidget.AddToViewport` _returnvalue_2 0)
            (set `PlayerController.bShowMouseCursor` true _returnvalue)
            (`GameplayStatics.SetGamePaused` false)
            (`WidgetBlueprintLibrary.SetInputMode_UIOnlyEx` _returnvalue))
          (:`then_1`
            (`/Engine/EditorBlueprintResources/StandardMacros.DoOnce` false
              (:`Completed`
                (`GameplayStatics.PlaySound2D` "/Game/Audio/VoiceOver/Murder_Begone_SelfVoice_getOut_master.Murder_Begone_SelfVoice_getOut_master")))))))))

(event `self.ReceiveActorBeginOverlap`
  (params (OtherActor :type "Actor Object Reference"))
  (`KismetSystemLibrary.PrintText` "Exit ?")
  (`self.EnableInput` (`GameplayStatics.GetPlayerController` 0))
  (goto _label :!via `Open`))

(fn `UserConstructionScript`)